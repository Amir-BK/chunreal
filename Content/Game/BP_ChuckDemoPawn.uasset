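; Player pawn for a Chuck demo that highlights interactables and lets the player use in-world code editor widgets.
; Each tick it line-traces from the camera and sends a highlight message to the hit component.
; Left click drives WidgetInteraction; on a WBP_ChuckCodeEditor it switches to UI-only input and blends the view to that widget's actor, returning when focus releases.
; Mouse release frees any held interactable, but the grab logic is unwired.
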(event Custom|CustomEvent
  (EventDispatchers|UnbindEventfromOnWidgetFocusRelease (stale Input|MouseEvents|LeftMouseButton _output_get) (delegate Custom|CustomEvent))
  (Game|Player|SetViewTargetwithBlend (Game|GetPlayerController 0) self 0.5 "VTBlend_Linear" 0.0 false))

(event EventBeginPlay)

(event Collision|EventActorBeginOverlap
  (params (OtherActor :type Actor%20Object%20Reference)))

(event EventTick
  (params (DeltaSeconds :type Float%20%28single-precision%29))
  (bind _returnvalue (Game|GetPlayerController 0))
  (bind _playercameramanager (Variables|/Script/Engine.PlayerController|GetPlayerCameraManager _returnvalue))
  (bind _returnvalue_2 (Camera|GetCameraLocation _playercameramanager))
  (bind (_outhit _returnvalue_3) (Collision|LineTraceForObjects _returnvalue_2 (+ (* (Math|Vector|GetForwardVector (Camera|GetCameraRotation _playercameramanager)) 1.5e+03) _returnvalue_2) (Utilities|Array|MakeArray "ObjectTypeQuery2" "ObjectTypeQuery4") false 0 "None"))
  (if _returnvalue_3
    (Class|BPISimpleInteractions|DrawInteractorHighlight(Message) (.HitComponent (Collision|BreakHitResult _outhit)) (.ImpactPoint (Collision|BreakHitResult _outhit)))
    (Variables|Default|SetHit%20Component (.HitComponent (Collision|BreakHitResult _outhit)))
    (else
      (Variables|Default|SetHit%20Component 0))))

(event Input|MouseEvents|LeftMouseButton
  (params (Key :type Key%20Structure))
  (bind _returnvalue (Game|GetPlayerController 0))
  (bind _widgetinteraction (Variables|Default|GetWidgetInteraction))
  (bind _returnvalue_2 (Class|WidgetInteractionComponent|GetHoveredWidgetComponent _widgetinteraction))
  (bind _returnvalue_3 (UserInterface|GetWidget _returnvalue_2))
  (:Pressed
    (Class|WidgetInteractionComponent|PressPointerKey _widgetinteraction Key)
    (bind _aswbp_chuck_code_editor (Utilities|Casting|CastToWBP_ChuckCodeEditor _returnvalue_3))
    (bind _output_get (Variables|Default|SetAs%20WBP%20Chuck%20Code%20Editor _aswbp_chuck_code_editor))
    (Input|SetInputModeUIOnly _returnvalue _returnvalue_3 "DoNotLock" false)
    (Game|Player|SetViewTargetwithBlend _returnvalue (Components|GetOwner _returnvalue_2) 1.0 "VTBlend_Linear" 0.0 false)
    (EventDispatchers|BindEventtoOnWidgetFocusRelease _output_get (delegate Custom|CustomEvent)))
  (:Released
    (Class|WidgetInteractionComponent|ReleasePointerKey _widgetinteraction Key)
    (if (Utilities|IsValidInterface (Variables|Default|GetInteractable))
      (Default|Release (Variables|Default|GetInteractable))
      (Variables|Default|SetInteractable 0))))

(fn ConstructionScript)

(fn GetGrabLocation
  (return (Transformation|GetWorldTransform (Variables|Default|GetGrabLocation))))