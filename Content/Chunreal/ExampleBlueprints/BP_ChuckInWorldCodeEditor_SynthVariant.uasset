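; Example in-world ChucK live-code editor actor that plays its code through a synth component.
; The construction script hands the ChuckCode asset to the live-code widget component.
; On BeginPlay it spawns a ChucK instance from that code, initializes and activates ChuckSynth with it, and subscribes to the "Test" global event.
; A callback event prints global event names, widget unfocus is forwarded, and older widget-setup nodes remain disconnected.
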(event OnChuckWidgetUnfocus(ChuckLiveCodeWidget)
  (Default|CallChuckWidgetUnfocus))

(event Custom|Global%20Event%20Callback
  (params (GlobalEventName :type String))
  (Development|PrintString GlobalEventName))

(event EventBeginPlay
  (bind _returnvalue (Class|ChuckCode|SpawnChuckInstance (Variables|Default|GetChuckCode)))
  (bind _output_get (Variables|Default|SetNewVar_0 _returnvalue))
  (Class|ChuckSynthComponent|InitwithChuckInstance (Variables|Default|GetChuckSynth) _output_get)
  (Components|Activation|Activate (Variables|Default|GetChuckSynth) true)
  (Class|ChuckInstantiation|SubscribetoGlobalEvent _returnvalue "Test" (delegate Custom|Global%20Event%20Callback)))

(fn ConstructionScript
  (Variables|/Script/Chunreal.ChuckLiveCodeWidgetComponent|SetChuckCode (Variables|Default|GetChuckLiveCodeWidget) (Variables|Default|GetChuckCode)))