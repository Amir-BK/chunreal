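; Chunreal example actor that plays a ChucK-synthesized plucked-string sound when its physics sphere hits something.
; On each hit, it writes Karplus-Strong ChucK code into the audio component's string parameter and fires a trigger to run it.
; String replacement injects a delay length mapped from impulse magnitude, so impact strength changes pitch.
; The same magnitude, passed through a power curve, sets volume after the trigger.
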(event OnComponentHit(Sphere)
  (params (HitComponent :type Primitive%20Component%20Object%20Reference) (OtherActor :type Actor%20Object%20Reference) (OtherComp :type Primitive%20Component%20Object%20Reference) (NormalImpulse :type Vector :default "0, 0, 0") (Hit :type Hit%20Result%20Structure%20%28by%20ref%29))
  (bind _returnvalue (Math|Vector|VectorLength NormalImpulse))
  (bind _chunreal_audio (Variables|Default|GetChunreal_Audio))
  ;[1 1 1] Write ChucK code and Set Parameter using String Replacement
  ; (EM - 06/22/23)
  (Class|AudioParameterControllerInterface|SetStringParameter _chunreal_audio "ChuckCode1" (Utilities|String|Replace (Utilities|String|MakeLiteralString "// karplus + strong plucked string filter 
// Ge Wang (gewang@cs.princeton.edu) 
 
// feedforward 
Noise imp => OneZero lowpass => dac; 
// feedback 
lowpass => Delay delay => lowpass; 
 
// our radius 
.99999 => float R; 
// our delay order 
DELAYPARAM => float L; 
// set delay 
L::samp => delay.delay; 
// set dissipation factor 
Math.pow( R, L ) => delay.gain; 
// place zero 
-1 => lowpass.zero; 
 
// fire excitation 
0.5 => imp.gain; 
// for one delay round trip 
L::samp => now; 
// cease fire 
0 => imp.gain; 
 
// advance time 
(Math.log(.0001) / Math.log(R))::samp => now;") "DELAYPARAM" (Utilities|String|ToString(Float) (Math|Float|MapRangeClamped _returnvalue 2e+03 2e+05 3e+02 1e+03))))
  (Class|AudioParameterControllerInterface|SetTriggerParameter _chunreal_audio "TriggerChuck")
  (Audio|Components|Audio|SetVolumeMultiplier (Variables|Default|GetChunreal_Audio) (Math|Float|Power (Math|Float|MapRangeClamped _returnvalue 2e+03 2e+05 0.0 1.0) 1.5) :!class /Script/Engine.AudioComponent))

(event EventBeginPlay)

(event EventTick
  (params (DeltaSeconds :type Float%20%28single-precision%29)))

(fn ConstructionScript)