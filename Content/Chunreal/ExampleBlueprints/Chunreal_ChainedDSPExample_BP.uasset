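; Example Blueprint for Chunreal that runs two chained ChucK programs through a MetaSound source and visualizes the sound on a sphere.
; On BeginPlay it sends code strings, IDs and a wave asset to the audio component, then triggers ChucK and wave playback.
; A random-note sine generator feeds a stereo feedback echo.
; Each Tick, it reads the generator's global frequency by ID and maps it to the sphere's color.
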(event EventBeginPlay
  ;[1 1 1] Write ChucK code as string and compile. Set wave asset and play wave player.
  ; (EM - 06/22/23)
  ;;[1 1 1] Based on how the ChucK nodes are routed in the MetaSound source (ChainedDSPExample), the output of ChuckCode1 goes into the "adc" of ChuckCode2
  (Class|AudioParameterControllerInterface|SetStringParameter (Variables|Default|GetChunreal_Audio) "ChuckCode1" (Utilities|String|MakeLiteralString "SinOsc osc => dac; 
0 => global float freq; 
0.5 => osc.gain; 
 
// an array 
[ 0, 2, 4, 7, 9, 11 ] @=> int hi[]; 
 
while( true ) 
{ 
    Std.mtof( 45 + Math.random2(0,3) * 12 + hi[Math.random2(0,hi.size()-1)] ) => freq; 
    freq => osc.freq; 
    200::ms => now; 
}"))
  (Class|AudioParameterControllerInterface|SetStringParameter (Variables|Default|GetChunreal_Audio) "ChuckCode2" (Utilities|String|MakeLiteralString "// feedforward 
adc => Gain gL => dac.left; 
adc => Gain gR => dac.right; 
// feedback 
gL => Gain feedbackL => DelayL delayL => gL; 
gR => Gain feedbackR => DelayL delayR => gR; 
 
// set delay parameters 
.75::second => delayL.max => delayL.delay; 
.95::second => delayR.max => delayR.delay; 
// set feedback 
.5 => feedbackL.gain; 
.5 => feedbackR.gain; 
// set effects mix 
.75 => delayL.gain; 
.75 => delayR.gain; 
 
// infinite time loop 
while( true ) 1::second => now;"))
  (Class|AudioParameterControllerInterface|SetStringParameter (Variables|Default|GetChunreal_Audio) "ChuckID1" "MyCode1")
  (Class|AudioParameterControllerInterface|SetStringParameter (Variables|Default|GetChunreal_Audio) "ChuckID2" "MyCode2")
  (Class|AudioComponent|SetWaveParameter (Variables|Default|GetChunreal_Audio) "WaveAsset" (Variables|Default|GetwaveAsset))
  (Class|AudioParameterControllerInterface|SetTriggerParameter (Variables|Default|GetChunreal_Audio) "PlayWave")
  (Class|AudioParameterControllerInterface|SetTriggerParameter (Variables|Default|GetChunreal_Audio) "TriggerChuck"))

(event EventTick
  (params (DeltaSeconds :type Float%20%28single-precision%29))
  ;[1 1 1] Get ChucK global variable "freq" using assigned ID and map it to the sphere color
  (bind _returnvalue (Class|ChunrealBlueprint|GetChuckGlobalFloat "MyCode1" "freq"))
  (Rendering|Material|SetVectorParameterValueonMaterials (Variables|Default|GetSphere) "Color" (Math|Vector|MakeVector 0.0 0.0 (Math|Float|MapRangeClamped _returnvalue 1e+02 2e+03 0.0 255.0))))

(fn ConstructionScript)