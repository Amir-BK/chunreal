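; Chunreal example Blueprint that runs ChucK audio code in the world, named as an in-world code editor.
; On BeginPlay it spawns a ChucK instance from its code asset, prints the "Test" global event when fired, and plays a non-auto-destroying 2D sound that receives the instance as an audio parameter.
; The logic linking the code editor widget's text and compile button is disconnected, so it never runs.
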(event Custom|Global%20Event%20Callback
  (params (GlobalEventName :type String))
  (Development|PrintString GlobalEventName))

(event EventBeginPlay
  (bind _returnvalue (Class|ChuckCode|SpawnChuckInstance (Variables|Default|GetChuckCode)))
  (Class|ChuckInstantiation|SubscribetoGlobalEvent _returnvalue "Test" (delegate Custom|Global%20Event%20Callback))
  (bind _returnvalue_2 (Audio|SpawnSound2D "/Chunreal/Chunreal/ChuckInstancePlayer.ChuckInstancePlayer" 1.0 1.0 0.0 0 false false))
  (Variables|/Script/Engine.AudioComponent|SetDefaultParameters _returnvalue_2 (Utilities|Array|MakeArray (Class|AudioParameterConversionStatics|ObjecttoAudioParameter "Chuck Instance" _returnvalue) (Class|AudioParameterConversionStatics|FloattoAudioParameter "INC" 0.0)))
  (Audio|Components|Audio|Play _returnvalue_2 0.0))

(fn ConstructionScript)