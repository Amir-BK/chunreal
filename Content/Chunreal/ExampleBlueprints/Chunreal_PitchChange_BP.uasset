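; Example Blueprint for Chunreal that plays a ChucK script while sweeping its pitch, with a sphere material reacting in step.
; On BeginPlay it reads a .ck file from the project's ChuckFiles content folder, passes the code and an ID to the ChunrealAudio component as parameters, and triggers it.
; Each Tick, a slow sine of game time drives both the audio pitch multiplier and the sphere material's UV parameter.
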(event EventBeginPlay
  (bind _chunreal_audio (Variables|Default|GetChunreal_Audio))
  ;[1 1 1] Read ChucK code from /Content/ChuckFiles/hevymetl-dance-now.ck and compile. Assign ID(string) to ChuckID1
  ; (EM - 06/24/23)
  (Class|AudioParameterControllerInterface|SetStringParameter _chunreal_audio "ChuckCode1" (.text (Class|ChunrealBlueprint|ReadFile (Utilities|String|Append (Class|KismetSystemLibrary|GetProjectContentDirectory) "ChuckFiles/" "hevymetl-dance-now.ck"))))
  (Class|AudioParameterControllerInterface|SetStringParameter _chunreal_audio "ChuckID1" (Variables|Default|GetID))
  (Class|AudioParameterControllerInterface|SetTriggerParameter _chunreal_audio "TriggerChuck"))

(event EventTick
  (params (DeltaSeconds :type Float%20%28single-precision%29))
  (bind _returnvalue (Actor|GetGameTimeSinceCreation))
  (bind _returnvalue_2 (* _returnvalue 0.3))
  (bind _returnvalue_3 (Math|Trig|Sin(Radians) _returnvalue_2))
  ;[1 1 1] Oscillate pitch multiplier between 0.1 and 2, and map it to the material UV multiplier
  (Audio|Components|Audio|SetPitchMultiplier (Variables|Default|GetChunreal_Audio) (Math|Float|MapRangeClamped _returnvalue_3 -1.0 1.0 0.1 2.0))
  (Rendering|Material|SetScalarParameterValueonMaterials (Variables|Default|GetSphere) "UV" (Math|Float|MapRangeClamped _returnvalue_3 -1.0 1.0 1.0 2e+01)))

(fn ConstructionScript)